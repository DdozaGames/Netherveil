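; BP_QuestManager handles the ending cutscene that plays when the boss stage is cleared.
; On BeginPlay it hides two pairs of boss and player mesh actors that serve as stand-ins for sequences.
; PlaySequencerClearBossStage unhides the second pair, then creates a level sequence player for LS_ClearBossStage and plays it.
; The first pair is only hidden here, and no quest-tracking logic is present.
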(event EventBeginPlay
  ;[1 1 1] 시퀀스용 캐릭터 메시 숨기기
  (Rendering|SetActorHiddenInGame (Variables|Default|GetBossMesh0) true)
  (Rendering|SetActorHiddenInGame (Variables|Default|GetPlayerMesh0) true)
  (Rendering|SetActorHiddenInGame (Variables|Default|GetBossMesh1) true)
  (Rendering|SetActorHiddenInGame (Variables|Default|GetPlayerMesh1) true))

(event EventPlaySequencerClearBossStage
  ;[1 1 1] 엔딩씬 재생
  (Rendering|SetActorHiddenInGame (Variables|Default|GetBossMesh1) false)
  (Rendering|SetActorHiddenInGame (Variables|Default|GetPlayerMesh1) false)
  (bind _returnvalue (Sequencer|Player|CreateLevelSequencePlayer "/Game/Cinematics/LS_ClearBossStage.LS_ClearBossStage"))
  (Sequencer|Player|Play _returnvalue :!class /Script/MovieScene.MovieSceneSequencePlayer))

(fn ConstructionScript)