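; BP_StageTriggerVolume is a stage trigger volume that plays the boss-stage entrance cutscene.
; PlaySequencerEnterBossStage unhides the BossMesh and PlayerMesh actors, plays LS_EnterBossStage, then destroys both after a fixed delay rather than on a sequence-finished event.
; Nothing in this graph calls that event, and BeginPlay and overlap are empty.
; The initial mesh hiding and StageIndex debug print are disconnected.
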(event EventBeginPlay)

(event Collision|EventActorBeginOverlap
  (params (OtherActor :type Actor%20Object%20Reference)))

(event EventTick
  (params (DeltaSeconds :type Float%20%28single-precision%29)))

(event EventPlaySequencerEnterBossStage
  ;[1 1 1] 보스 입장 시퀀스 재생 & 스켈레탈 메시 visible관리
  (Rendering|SetActorHiddenInGame (Variables|Default|GetBossMesh) false)
  (Rendering|SetActorHiddenInGame (Variables|Default|GetPlayerMesh) false)
  (bind _returnvalue (Sequencer|Player|CreateLevelSequencePlayer "/Game/Cinematics/LS_EnterBossStage.LS_EnterBossStage"))
  (Sequencer|Player|Play _returnvalue :!class /Script/MovieScene.MovieSceneSequencePlayer)
  (Utilities|FlowControl|Delay 12.5)
  (Actor|DestroyActor (Variables|Default|GetBossMesh))
  (Actor|DestroyActor (Variables|Default|GetPlayerMesh)))

(fn ConstructionScript)