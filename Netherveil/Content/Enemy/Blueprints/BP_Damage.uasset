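; BP_Damage is a floating damage number actor in the enemy content that shows an amount, drifts away and removes itself.
; On BeginPlay it passes DamageAmount into its WBP_Damage widget and records start and end locations at a fixed offset, rising upward.
; A timeline lerps the actor between those points and destroys it when finished.
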(event EventBeginPlay
  (bind _aswbp_damage (Utilities|Casting|CastToWBP_Damage (UserInterface|GetWidget (Variables|Default|GetWidget))))
  (Variables|/Game/UI/WBP_Damage.WBP_Damage_C|SetDamageAmount _aswbp_damage (Variables|Default|GetDamage%20Amount))
  (bind _output_get (Variables|Default|SetstartLoc (Transformation|GetActorLocation)))
  (Variables|Default|SetendLoc (+ _output_get "-25.000000,-25.000000,50.000000"))
  (bind _move_track (Timeline|MoveT Play)
    (:Update
      (Transformation|SetActorLocation (Math|Vector|Lerp(Vector) (Variables|Default|GetstartLoc) (Variables|Default|GetendLoc) _move_track) false false))
    (:Finished
      (Actor|DestroyActor))))

(fn ConstructionScript)