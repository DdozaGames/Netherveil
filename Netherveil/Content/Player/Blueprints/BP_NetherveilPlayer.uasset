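; Netherveil player Blueprint that drives the HUD and stage-transition presentation on top of C++ parent logic.
; Events push health, ammo, weapon-swap and quest state into a UI_Screen widget, while Tick lerps quest and boss progress bars.
; Completing Rift1 spawns a stage portal, and game over swaps the HUD for a delayed game-over widget.
; Boss-stage entry hides and freezes the player until a timer restores them, moves them forward and shows the boss bar.
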(event Custom|EnterBossStage
  ;[1 1 1] 보스전 진입 시 시퀀스 재생 동안 플레이어 이동 X, 안보이게, MainUI visible
  (Pawn|Components|CharacterMovement|SetMovementMode (Variables|Character|GetCharacterMovement) "MOVE_Walking" 0)
  (Rendering|SetActorHiddenInGame false)
  (Widget|SetVisibility (Variables|/Game/UI/UI_Screen.UI_Screen_C|GetBossHP (Variables|Default|GetUI%20Screen)) "Visible")
  (Class|NetherveilPlayer|SetCrosshairUIVisible)
  (Transformation|SetActorLocation (+ (Transformation|GetActorLocation) (* (Transformation|GetActorForwardVector) "2000.000000,0.000000,0.000000")) false false)
  (Widget|SetVisibility (Variables|Default|GetUI%20Screen) "Visible"))

(event EventBeginPlay
  (bind _returnvalue (UserInterface|CreateWidget "/Game/UI/UI_Screen.UI_Screen_C" (Game|GetPlayerController 0)))
  (bind _output_get (Variables|Default|SetUI%20Screen _returnvalue))
  (UserInterface|Viewport|AddtoViewport _output_get 0)
  (Utilities|FlowControl|Delay 0.05)
  (CallFunction|UIctrlHP)
  (Class|NetherveilPlayer|OnUsingGrenade true)
  (CallFunction|UIctrlGrenadAmmo)
  (Utilities|IsValid (Variables|Default|GetUI%20Screen)
    (:Is%20Valid
      (Default|FullHPMessage (Variables|Default|GetUI%20Screen)))))

(event EventUpdateHpUI
  (CallFunction|UIctrlHP))

(event EventUpdateAmmoUI
  (CallFunction|UIctrlGrenadAmmo))

(event EventOnGameOver
  ;[1 1 1] 추가 안하면 c++에서 구현 내용 덮어써짐
  (|CallParentFunction)
  (Utilities|FlowControl|Delay 5.0)
  (Widget|SetVisibility (Variables|Default|GetUI%20Screen) "Hidden")
  (bind _returnvalue (UserInterface|CreateWidget "/Game/UI/WBP_GameOver.WBP_GameOver_C"))
  (UserInterface|Viewport|AddtoViewport _returnvalue 0))

(event EventOnUsingGrenade
  (params (isGrenade :type Boolean))
  (bind _ui_screen (Variables|Default|GetUI%20Screen))
  (Utilities|IsValid _ui_screen
    (:Is%20Valid
      (Variables|/Game/UI/UI_Screen.UI_Screen_C|SetisGrenaded _ui_screen isGrenade)
      (Default|SwapWeapon _ui_screen))))

(event EventDisplayFullHPMessage
  (bind _ui_screen (Variables|Default|GetUI%20Screen))
  (Utilities|IsValid _ui_screen
    (:Is%20Valid
      (Variables|/Game/UI/UI_Screen.UI_Screen_C|SetIsFullHP _ui_screen true)
      (Default|FullHPMessage _ui_screen)
      (Utilities|FlowControl|Delay 2.0)
      (Variables|/Game/UI/UI_Screen.UI_Screen_C|SetIsFullHP _ui_screen false)
      (Default|FullHPMessage _ui_screen))))

(event EventEnterNewStageUI
  (params (stageIndex :type Integer))
  (bind _ui_screen (Variables|Default|GetUI%20Screen))
  (bind _missionui (Variables|/Game/UI/UI_Screen.UI_Screen_C|GetMissionUI _ui_screen))
  (if (== stageIndex 2)
    ;[1 1 1] 보스전 진입 시 시퀀스 재생 동안 플레이어 이동 X, 안보이게, MainUI visible
    (Widget|SetVisibility (Variables|Default|GetUI%20Screen) "Hidden")
    (Class|NetherveilPlayer|SetCrosshairUIhidden)
    (Pawn|Components|CharacterMovement|DisableMovement (Variables|Character|GetCharacterMovement))
    (Rendering|SetActorHiddenInGame true)
    (Utilities|Time|SetTimerbyEvent (delegate Custom|EnterBossStage) 12.5)
    (else
      ;[1 1 1] stage 1,2 입장 시 뜨는 UI
      (Variables|/Script/UMG.TextBlock|SetText _missionui (Utilities|Text|ToText(String) (Utilities|String|Append "Stage " (Utilities|String|ToString(Integer) (+ stageIndex 1)) " 입장")))
      (Widget|SetVisibility _missionui "Visible")
      (Utilities|FlowControl|Delay 2.0)
      (Widget|SetVisibility _missionui "Hidden"))))

(event EventTick
  (params (DeltaSeconds :type Float%20%28single-precision%29))
  (CallFunction|UIctrlQuest)
  ;[1 0.838 0] 보스전일때만
  (if true
    (CallFunction|UIctrlBossHP)))

(event EventCompleteQuestUI
  (params (RiftID :type Name :default "None"))
  (Utilities|FlowControl|Sequence
    (:then_0
      (if (== RiftID "Rift1")
        (Default|CompleteQuest1 (Variables|Default|GetUI%20Screen))
        ;[1 0.553 0] stage 1->2 이동 포탈
        (Game|SpawnActorfromClass "/Game/Quest/BP_StagePortal.BP_StagePortal_C" (Math|Transform|MakeTransform "-52529.563699,-14042.137898,-5183.605880" "0, 0, 0" "1.000000,1.000000,1.000000") "Undefined" "MultiplyWithRoot" 0 0)))
    (:then_1
      (if (== RiftID "Rift2")
        (Default|CompleteQuest2 (Variables|Default|GetUI%20Screen))))
    (:then_2
      (if (== RiftID "Rift3")
        (Default|CompleteQuest3 (Variables|Default|GetUI%20Screen))))))

(fn ConstructionScript)

(fn UIctrlHP
  (Variables|/Game/UI/UI_Screen.UI_Screen_C|SethpRatio (Variables|Default|GetUI%20Screen) (/ (Math|Conversions|ToFloat(Integer) (Variables|Default|Gethp)) (Math|Conversions|ToFloat(Integer) (Variables|Default|GetinitialHp))))
  (Variables|/Game/UI/UI_Screen.UI_Screen_C|SethpString (Variables|Default|GetUI%20Screen) (Utilities|String|Append (Utilities|String|ToString(Integer) (Variables|Default|Gethp)) "/" (Utilities|String|ToString(Integer) (Variables|Default|GetinitialHp)))))

(fn UIctrlGrenadAmmo
  (Variables|/Game/UI/UI_Screen.UI_Screen_C|SetCurrentAmmo_Grenade (Variables|Default|GetUI%20Screen) (Utilities|String|ToString(Integer) (Variables|Default|GetgrenadeCurrentAmmo)))
  (Variables|/Game/UI/UI_Screen.UI_Screen_C|SetRemainingAmmo_Grenade (Variables|Default|GetUI%20Screen) (Utilities|String|ToString(Integer) (Variables|Default|GetgrenadeRemaingAmmo)))
  (Variables|/Game/UI/UI_Screen.UI_Screen_C|SetCurrentAmmo_Sniper (Variables|Default|GetUI%20Screen) (Utilities|String|ToString(Integer) (Variables|Default|GetsniperCurrentAmmo)))
  (Variables|/Game/UI/UI_Screen.UI_Screen_C|SetRemainingAmmo_Sniper (Variables|Default|GetUI%20Screen) (Utilities|String|ToString(Integer) (Variables|Default|GetsniperRemaingAmmo))))

(fn UIctrlQuest
  (bind _ui_screen (Variables|Default|GetUI%20Screen))
  (bind _questprogress (Variables|Default|GetquestProgress))
  (Variables|/Game/UI/UI_Screen.UI_Screen_C|SetQuestRatio _ui_screen (Math|Float|Lerp (Variables|/Game/UI/UI_Screen.UI_Screen_C|GetQuestRatio _ui_screen) _questprogress 0.1))
  (Variables|/Game/UI/UI_Screen.UI_Screen_C|SetQuestString _ui_screen (Utilities|String|Append (Utilities|String|ToString(Text) (Utilities|Text|ToText(Float) (* _questprogress 1e+02) "HalfToEven" false true 1 324 3)) "%")))

(fn UIctrlBossHP
  (bind _ui_screen (Variables|Default|GetUI%20Screen))
  (Variables|/Game/UI/UI_Screen.UI_Screen_C|SetBossRatio _ui_screen (Math|Float|Lerp (Variables|/Game/UI/UI_Screen.UI_Screen_C|GetBossRatio _ui_screen) (Variables|Default|GetbossProgress) 0.1)))